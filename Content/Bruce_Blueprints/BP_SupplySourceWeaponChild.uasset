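; Weapon supply cache child Blueprint that places itself via SetLocation on BeginPlay and visually shrinks as it is used.
; The construction script scales the WeaponSupply component by cache array size.
; On overlap, it shrinks one step after a delay while CachesAvailable is non-empty.
; Otherwise it destroys itself, with a delayed relocate and respawn of its class wired after the DestroyActor call.
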(event Custom|SizeDecrease
  ;[1 1 1] SizeDecrease Custom Event
  ;;[1 1 1] Checking for available caches
  (if (!= (Utilities|Array|Length (Variables|Default|GetCachesAvailable)) 0)
    ;;[1 1 1] Decreasing scale of cache
    (Utilities|FlowControl|Delay 4.0)
    (CallFunction|DecrementScale)
    (else
      ;;[1 1 1] Respawning Actor in Game
      (Actor|DestroyActor)
      (Utilities|FlowControl|Delay 3e+01)
      (CallFunction|SetLocation)
      (Game|SpawnActorfromClass "BP_SupplySourceWeaponChild_C" (Math|Transform|MakeTransform (Variables|Default|GetcacheLocation) "0, 0, 0" "1,1,1") "Undefined" 0 0))))

(event EventBeginPlay
  (|CallParentFunction)
  (CallFunction|SetLocation))

(event Collision|EventActorBeginOverlap
  (params (OtherActor :type Actor%20Object%20Reference))
  (|CallParentFunction OtherActor)
  (CallFunction|SizeDecrease))

(event EventTick
  (params (DeltaSeconds :type Float%20%28single-precision%29))
  (|CallParentFunction DeltaSeconds) ; This node is disabled and will not be called.\nDrag off pins to build functionality.
)

(fn ConstructionScript
  (|CallParentFunction)
  ;[1 1 1] Setting the scale
  (bind _output_get (Variables|Default|SetcurrentScale (+ (Variables|Default|GetbaseScale) (* "0.250000,0.250000,0.250000" (Variables|Default|GetsizeOfCacheArray)))))
  (Transformation|SetWorldScale3D (Variables|Default|GetWeaponSupply) _output_get))

(fn DecrementScale
  (bind _output_get (Variables|Default|SetcurrentScale (- (Variables|Default|GetcurrentScale) "0.250000,0.250000,0.250000")))
  (Transformation|SetWorldScale3D (Variables|Default|GetWeaponSupply) _output_get))
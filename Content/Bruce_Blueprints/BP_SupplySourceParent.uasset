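; Supply source parent Blueprint, judging by its name, that tracks a limited stock of item caches.
; Construction fills a boolean array with 3 to 5 true entries as the stock count.
; Any actor overlap calls GiveItemToCollector, which only decrements stock by setting the last entry false and removing it.
; A SetLocation event, not called here, stores a random LocationArray entry in CacheLocation without moving the actor.
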(event Custom|SetLocation
  ;[1 1 1] SetLocation Custom Event
  (bind _output_get (Variables|Default|Setindex (Math|Random|RandomIntegerinRange 0 (- (Utilities|Array|Length (Variables|Default|GetLocationArray)) 1))))
  (if (Utilities|Array|IsValidIndex (Variables|Default|GetLocationArray) _output_get)
    (Variables|Default|SetcacheLocation (Utilities|Array|Get(acopy) (Variables|Default|GetLocationArray) (Variables|Default|Getindex)))))

(event Custom|GiveItemToCollector
  ;[1 1 1] Give Item To Collector Custom Event
  (CallFunction|DecrementCachesAvailable))

(event EventBeginPlay)

(event Collision|EventActorBeginOverlap
  (params (OtherActor :type Actor%20Object%20Reference))
  (CallFunction|GiveItemtoCollector))

(event EventTick
  (params (DeltaSeconds :type Float%20%28single-precision%29)))

(fn ConstructionScript
  ;[1 1 1] Defaulting cacheItem to true
  (Variables|Default|SetcacheItem true)
  ;[1 1 1] Setting random size of Cache Array between 3 and 5 units
  (bind _output_get (Variables|Default|SetsizeOfCacheArray (Math|Random|RandomIntegerinRange 3 5)))
  ;[1 1 1] Adding elements to CachesAvailable array
  (while (< (Utilities|Array|Length (Variables|Default|GetCachesAvailable)) _output_get)
    (Utilities|Array|Add (Variables|Default|GetCachesAvailable) (Variables|Default|GetcacheItem))))

(fn DecrementCachesAvailable
  (bind _cachesavailable (Variables|Default|GetCachesAvailable))
  ;[1 1 1] Setting cacheItem to false
  (bind _output_get (Variables|Default|SetcacheItem false))
  ;[1 1 1] Setting last element in array to false and removing from array
  (Utilities|Array|SetArrayElem _cachesavailable (Utilities|Array|LastIndex _cachesavailable) _output_get)
  (Utilities|Array|RemoveItem (Variables|Default|GetCachesAvailable) (Variables|Default|GetcacheItem)))